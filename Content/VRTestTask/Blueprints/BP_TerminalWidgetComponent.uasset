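; Widget component on a ticket terminal that bridges the WBP_Terminal UI and its owning BP_Terminal actor.
; On BeginPlay it binds to the widget's ticket purchase event and the terminal's credit card payment event.
; A purchase passes the destination to the terminal through SpawnTicket, then notifies the widget.
; A card payment on the terminal is relayed to the widget's OnPayment.
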(event Custom|OnCreditCartPay_Event
  (bind _returnvalue (CallFunction|GetTerminalWidget))
  (Utilities|IsValid _returnvalue
    (:Is%20Valid
      (Default|OnPayment _returnvalue))))

(event Custom|OnTickedPurchase_Event
  (params (DestinationName :type Name))
  (bind _returnvalue (CallFunction|GetTerminalWidget))
  (CallFunction|SpawnTicket DestinationName)
  (Utilities|IsValid _returnvalue
    (:Is%20Valid
      (Default|OnTicketPurchased _returnvalue))))

(event EventBeginPlay
  (bind _returnvalue (CallFunction|GetTerminalWidget))
  (Utilities|FlowControl|Sequence
    (:then_0
      (Utilities|IsValid _returnvalue
        (:Is%20Valid
          (EventDispatchers|AssignOnTickedPurchase _returnvalue (delegate Custom|OnTickedPurchase_Event)))))
    (:then_1
      (bind _asbp_terminal (Utilities|Casting|CastToBP_Terminal (Components|GetOwner)))
      (EventDispatchers|AssignOnCreditCartPay _asbp_terminal (delegate Custom|OnCreditCartPay_Event)))))

(fn GetTerminalWidget
  (bind _aswbp_terminal (Utilities|Casting|CastToWBP_Terminal (UserInterface|GetWidget)))
  (return _aswbp_terminal))

(fn GetOwnerTerminal
  (bind _asbp_terminal (Utilities|Casting|CastToBP_Terminal (Components|GetOwner)))
  (return _asbp_terminal))

(fn SpawnTicket
  (params (TicketDestination :type Name))
  (bind _returnvalue (CallFunction|GetOwnerTerminal))
  (Utilities|IsValid _returnvalue
    (:Is%20Valid
      (Default|OnTickedPurchased _returnvalue TicketDestination))))