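; BP_Turnstile is a ticket-checked turnstile that opens when an overlapping BP_Ticket's destination matches its own.
; A timeline drives a rotation lerp, applied negated to the left arm and directly to the right in world space.
; A Delay on the timeline's Update pin, rather than Finished, reverses the timeline after OpenTime to close it.
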(event OnComponentBeginOverlap(TurnstileTrigger)
  (params (OverlappedComponent :type Primitive%20Component%20Object%20Reference) (OtherActor :type Actor%20Object%20Reference) (OtherComp :type Primitive%20Component%20Object%20Reference) (OtherBodyIndex :type Integer) (bFromSweep :type Boolean) (SweepResult :type Hit%20Result%20Structure%20%28by%20ref%29))
  (bind _asbp_ticket (Utilities|Casting|CastToBP_Ticket OtherActor))
  (if (CallFunction|CheckTicketDestination _asbp_ticket)
    (CallFunction|OpenTurnstile)))

(event Custom|OpenTurnstile
  (bind _newtrack_0 (Timeline|Timeline Play)
    (:Update
      (CallFunction|SetTurnstilesRotation (Math|Rotator|Lerp(Rotator) "0, 0, 0" (Variables|Default|GetTurnstilesOpenRotation) _newtrack_0))
      (Utilities|FlowControl|Delay (Variables|Default|GetOpenTime))
      (CallFunction|CloseTurnstile))))

(event Custom|CloseTurnstile
  (bind _newtrack_0 (Timeline|Timeline Reverse)
    (:Update
      (CallFunction|SetTurnstilesRotation (Math|Rotator|Lerp(Rotator) "0, 0, 0" (Variables|Default|GetTurnstilesOpenRotation) _newtrack_0))
      (Utilities|FlowControl|Delay (Variables|Default|GetOpenTime))
      (CallFunction|CloseTurnstile))))

(fn ConstructionScript)

(fn SetTurnstilesRotation
  (params (NewRotation :type Rotator))
  (Utilities|FlowControl|Sequence
    (:then_0
      (Utilities|IsValid (Variables|Default|GetTurnstileLeft)
        (:Is%20Valid
          (Transformation|SetWorldRotation (Variables|Default|GetTurnstileLeft) (Class|KismetMathLibrary|NegateRotator NewRotation) false false))))
    (:then_1
      (Utilities|IsValid (Variables|Default|GetTurnstileRight)
        (:Is%20Valid
          (Transformation|SetWorldRotation (Variables|Default|GetTurnstileRight) NewRotation false false))))))

(fn CheckTicketDestination
  (params (Ticket :type BP%20Ticket%20Object%20Reference))
  (Utilities|IsValid Ticket
    (:Is%20Valid
      (return (Utilities|Enum|Equal(Enum) (Default|GetTicketDestination Ticket) (Variables|Default|GetDestination))))))