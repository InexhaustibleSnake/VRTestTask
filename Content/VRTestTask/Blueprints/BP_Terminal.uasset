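; BP_Terminal is a payment terminal that detects a credit card and dispenses tickets.
; An actor of CreditCardClass overlapping CreditCardTrigger fires the OnCreditCartPay dispatcher; OnCreditCardTriggerOverlap repeats this check as a function with an added validity test.
; OnTickedPurchased spawns a BP_Ticket with the given destination at TicketsSpawnPoint, falling back to the world origin if that point is invalid.
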(event OnComponentBeginOverlap(CreditCardTrigger)
  (params (OverlappedComponent :type Primitive%20Component%20Object%20Reference) (OtherActor :type Actor%20Object%20Reference) (OtherComp :type Primitive%20Component%20Object%20Reference) (OtherBodyIndex :type Integer) (bFromSweep :type Boolean) (SweepResult :type Hit%20Result%20Structure%20%28by%20ref%29))
  (if (Class|GameplayStatics|ObjectIsA OtherActor (Variables|Default|GetCreditCardClass))
    (Default|CallOnCreditCartPay)))

(fn ConstructionScript)

(fn OnCreditCardTriggerOverlap
  (params (OverlapActor :type Actor%20Object%20Reference))
  (if (and (Utilities|IsValid OverlapActor) (Class|GameplayStatics|ObjectIsA OverlapActor (Variables|Default|GetCreditCardClass)))
    (Default|CallOnCreditCartPay)))

(fn OnTickedPurchased
  (params (TicketDestination :type BE_Destinations%20Enum%20%28by%20ref%29 :default "NewEnumerator2"))
  (Game|SpawnActorfromClass "/Game/VRTestTask/Blueprints/Items/BP_Ticket.BP_Ticket_C" (Math|Transform|SelectTransform (Transformation|GetWorldTransform (Variables|Default|GetTicketsSpawnPoint)) (Math|Transform|MakeTransform "0, 0, 0") (Utilities|IsValid (Variables|Default|GetTicketsSpawnPoint))) "Undefined" "MultiplyWithRoot" 0 TicketDestination 0))