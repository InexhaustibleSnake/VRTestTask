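; BP_PlayerCharacter is the player character for a VR test project, handling locomotion, turning and hand grabbing.
; On BeginPlay with an HMD enabled, it sets floor-level tracking, sets pixel density and lowers the Scene component by BaseEyeHeight.
; Movement follows the Camera's forward and right vectors, while yaw input is scaled by RotationScale.
; Left and right grab presses call Grab on the matching hand; no release input is handled here.
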(event EventBeginPlay
  (if (Class|HeadMountedDisplayFunctionLibrary|IsHeadMountedDisplayEnabled)
    (Class|HeadMountedDisplayFunctionLibrary|SetTrackingOrigin "Floor")
    (Development|ExecuteConsoleCommand "vr.PixelDensity 1.0" 0)
    (Transformation|AddLocalOffset (Variables|Default|GetScene) (Math|Vector|MakeVector 0.0 0.0 (* (Variables|Default|GetBaseEyeHeight) -1.0)) false false)))

(event Input|ActionEvents|InputActionLeftArmGrab
  (params (Key :type Key%20Structure :default "None"))
  (:Pressed
    (Utilities|IsValid (Variables|Default|GetLeftHand)
      (:Is%20Valid
        (Default|Grab (Variables|Default|GetLeftHand))))))

(event Input|ActionEvents|InputActionRightArmGrab
  (params (Key :type Key%20Structure :default "None"))
  (:Pressed
    (Utilities|IsValid (Variables|Default|GetRightHand)
      (:Is%20Valid
        (Default|Grab (Variables|Default|GetRightHand))))))

(event Input|AxisEvents|InputAxisMoveForward
  (params (AxisValue :type Float%20%28single-precision%29))
  (Utilities|IsValid (Variables|Default|GetCamera)
    (:Is%20Valid
      (Pawn|Input|AddMovementInput (Math|Vector|GetForwardVector (Variables|Default|GetCamera)) AxisValue false))))

(event Input|AxisEvents|InputAxisMoveRight
  (params (AxisValue :type Float%20%28single-precision%29))
  (Utilities|IsValid (Variables|Default|GetCamera)
    (:Is%20Valid
      (Pawn|Input|AddMovementInput (Math|Vector|GetRightVector (Variables|Default|GetCamera)) AxisValue false))))

(event Input|AxisEvents|InputAxisRotateYaw
  (params (AxisValue :type Float%20%28single-precision%29))
  (Pawn|Input|AddControllerYawInput (* AxisValue (Variables|Default|GetRotationScale))))

(fn ConstructionScript)